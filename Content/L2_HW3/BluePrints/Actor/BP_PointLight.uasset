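; BP_PointLight is a point light actor that a linked button toggles on and off.
; On BeginPlay it checks that ControlButton is valid and binds its Switch event to the button's pressed event.
; Switch reads the PointLight component's visibility as the on/off state and calls SwitchOn or SwitchOff, which set that visibility.
; IsSwitchOn exposes the same state by wrapping IsOn.
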(event Custom|Switch
  ;[1 1 1] Actions after button click
  (if (CallFunction|Ison)
    (CallFunction|SwitchOff)
    (else
      (CallFunction|Switchon))))

(event EventBeginPlay
  ;[1 1 1] Check valid link Button and Binding his Event
  (bind _controlbutton (Variables|Default|GetControlButton)
    (:then
      (EventDispatchers|BindEventtoOnPressed _controlbutton (delegate Custom|Switch)))
    (:else)))

(event EventSwitchOff
  ;[1 1 1] Set light state OFF
  (Rendering|SetVisibility (Variables|Default|GetPointLight) false false))

(event EventSwitchon
  ;[1 1 1] Set light state ON
  (Rendering|SetVisibility (Variables|Default|GetPointLight) true false))

(fn ConstructionScript)

(fn Ison
  (return (Variables|/Script/Engine.SceneComponent|GetbVisible (Variables|Default|GetPointLight))))

(fn IsSwitchon
  (return (CallFunction|Ison)))