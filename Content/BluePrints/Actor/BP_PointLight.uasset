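; BP_PointLight is a point light actor that can be toggled on and off by a linked control button.
; On BeginPlay it binds Switch to the pressed event of ControlButton, if that reference is valid.
; Switch checks the PointLight component's visibility through IsOn, then calls SwitchOn or SwitchOff to flip it.
; IsSwitchOn also reports the light's state by returning IsOn.
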(event Custom|Switch
  (if (CallFunction|Ison)
    (CallFunction|SwitchOff)
    (else
      (CallFunction|Switchon))))

(event EventBeginPlay
  (bind _controlbutton (Variables|Default|GetControlButton)
    (:then
      (EventDispatchers|BindEventtoOnPressed _controlbutton (delegate Custom|Switch)))
    (:else)))

(event EventSwitchOff
  (Rendering|SetVisibility (Variables|Default|GetPointLight) false false))

(event EventSwitchon
  (Rendering|SetVisibility (Variables|Default|GetPointLight) true false))

(fn ConstructionScript)

(fn Ison
  (return (Variables|/Script/Engine.SceneComponent|GetbVisible (Variables|Default|GetPointLight))))

(fn IsSwitchon
  (return (CallFunction|Ison)))